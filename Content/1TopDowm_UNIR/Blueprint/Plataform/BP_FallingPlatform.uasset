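; Falling platform that drops under physics a set time after the top-down player character steps into its trigger box.
; The box overlap starts a countdown on Tick; at zero it destroys the InterpToMovement, Spline and Box components and enables physics simulation on the mesh.
; A ColorLerp parameter is set once per overlap on a dynamic material instance, but the mesh is assigned the base M_Platform instead.
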(event OnComponentBeginOverlap(Box)
  (params (OverlappedComponent :type Primitive%20Component%20Object%20Reference) (OtherActor :type Actor%20Object%20Reference) (OtherComp :type Primitive%20Component%20Object%20Reference) (OtherBodyIndex :type Integer) (bFromSweep :type Boolean) (SweepResult :type Hit%20Result%20Structure%20%28by%20ref%29))
  (Utilities|Casting|CastToBP_TopDown_Character_UNIR OtherActor)
  (Variables|Default|SetbStarCountdown true)
  (Rendering|Material|SetScalarParameterValue (Variables|Default|GetDynamicMaterial) "ColorLerp" (/ (Variables|Default|Gettimer) (Variables|Default|GetTimetoFall)) :!class /Script/Engine.MaterialInstanceDynamic))

(event EventBeginPlay
  (|CallParentFunction)
  (bind _returnvalue (Rendering|Material|CreateDynamicMaterialInstance "/Game/1TopDowm_UNIR/FX/Platform/M_Platform.M_Platform" "None" "None" :!class /Script/Engine.KismetMaterialLibrary))
  (Variables|Default|SetDynamicMaterial _returnvalue)
  (Rendering|Material|SetMaterial (Variables|Default|GetSM_Modules_Platform) 2 "/Game/1TopDowm_UNIR/FX/Platform/M_Platform.M_Platform")
  (Variables|Default|SetTimetoFall (Variables|Default|Gettimer))
  (Variables|Default|SetPositionIni (Transformation|GetWorldLocation (Variables|Default|GetSM_Modules_Platform))))

(event Collision|EventActorBeginOverlap
  (params (OtherActor :type Actor%20Object%20Reference))
  (|CallParentFunction OtherActor))

(event EventTick
  (params (DeltaSeconds :type Float%20%28single-precision%29))
  (|CallParentFunction DeltaSeconds)
  (if (Variables|Default|GetbStarCountdown)
    (Variables|Default|Settimer (- (Variables|Default|Gettimer) DeltaSeconds))
    (if (<= (Variables|Default|Gettimer) 0.0)
      (Variables|Default|SetbStarCountdown false)
      (Components|DestroyComponent (Variables|Default|GetInterpToMovement))
      (Physics|SetSimulatePhysics (Variables|Default|GetSM_Modules_Platform) true))))

(fn ConstructionScript
  (|CallParentFunction))