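; BP_EnemyGuard is a simple AI guard for a top-down game that patrols, chases the player and calls the player's Chekpoint function on overlap.
; Patrol loops AIMoveTo between random TargetPoints sharing its tag, pausing briefly after each arrival.
; AIPerception updates send it running after the player or toward the location of a "ball"-tagged stimulus.
; When perception forgets a target, it logs that, slows down and resumes patrolling.
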(event OnTargetPerceptionUpdated(AIPerception)
  (params (Actor :type Actor%20Object%20Reference) (Stimulus :type AI%20Stimulus%20Structure))
  (bind (_age _expirationage _strength _stimuluslocation _receiverlocation _tag) (Utilities|Struct|BreakAIStimulus Stimulus))
  (if (not (== _tag "ball"))
    (bind _asbp_top_down_character_unir (Utilities|Casting|CastToBP_TopDown_Character_UNIR Actor))
    (Variables|/Script/Engine.CharacterMovementComponent|SetMaxWalkSpeed (Variables|Character|GetCharacterMovement) 4e+02)
    (AI|AIMoveTo self "0, 0, 0" _asbp_top_down_character_unir 5.0 false)
    (else
      (AI|AIMoveTo self _stimuluslocation 0 5.0 false))))

(event OnTargetPerceptionForgotten(AIPerception)
  (params (Actor :type Actor%20Object%20Reference))
  (Variables|/Script/Engine.CharacterMovementComponent|SetMaxWalkSpeed (Variables|Character|GetCharacterMovement) 2e+02)
  (bind _outactors (Actor|GetAllActorsOfClasswithTag "/Script/Engine.TargetPoint" (Variables|Default|GetTag) :!label _label))
  (AI|AIMoveTo self "0, 0, 0" (.OutItem (Utilities|Array|Random _outactors)) 5.0 false
    (:OnSuccess
      (Utilities|FlowControl|Delay 1.0)
      (goto _label))))

(event Custom|OnTargetPerceptionForgotten_Event
  (params (Actor :type Actor%20Object%20Reference))
  (Development|PrintString (Utilities|String|ToString(Text) (Utilities|Text|FormatText "AI Forget this {actor}" Actor))))

(event EventBeginPlay
  (EventDispatchers|AssignOnTargetPerceptionForgotten (Variables|Default|GetAIPerception) (delegate Custom|OnTargetPerceptionForgotten_Event))
  (bind _outactors (Actor|GetAllActorsOfClasswithTag "/Script/Engine.TargetPoint" (Variables|Default|GetTag) :!label _label))
  (AI|AIMoveTo self "0, 0, 0" (.OutItem (Utilities|Array|Random _outactors)) 5.0 false
    (:OnSuccess
      (Utilities|FlowControl|Delay 1.0)
      (goto _label))))

(event Collision|EventActorBeginOverlap
  (params (OtherActor :type Actor%20Object%20Reference))
  (bind _asbp_top_down_character_unir (Utilities|Casting|CastToBP_TopDown_Character_UNIR OtherActor))
  (Default|Chekpoint _asbp_top_down_character_unir))

(fn ConstructionScript)