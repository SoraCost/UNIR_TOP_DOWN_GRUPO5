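; BP_inventory manages the player's ten-slot item inventory, with I toggling its widget on screen.
; E runs a sphere trace just below the player's location to find a BP_item.
; A slot loop stacks it up to 64 or fills an empty slot, whichever qualifies first.
; Each pickup plays a sound, reloads the widget and destroys the item, whose validity check guards the remaining iterations.
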(event EventBeginPlay
  (bind _returnvalue (UserInterface|CreateWidget "/Game/1TopDowm_UNIR/inventory/widgets/Wd_widgetInventory.Wd_widgetInventory_C"))
  (Variables|Default|Setwidgetinventory _returnvalue)
  (Utilities|Array|Resize (Variables|Default|Getitems) 10)
  (Default|LoadInventory (Variables|Default|Getwidgetinventory) self))

(event EventTick
  (params (DeltaSeconds :type Float%20%28single-precision%29)))

(event Input|KeyboardEvents|I
  (params (Key :type Key%20Structure))
  (bind _widgetinventory (Variables|Default|Getwidgetinventory))
  (:Pressed
    (if (Widget|IsVisible (Variables|Default|Getwidgetinventory))
      (Widget|RemovefromParent _widgetinventory)
      (else
        (UserInterface|Viewport|AddtoViewport _widgetinventory 0)))))

(event Input|KeyboardEvents|E
  (params (Key :type Key%20Structure))
  (bind _returnvalue (Game|GetPlayerCharacter 0))
  (bind _returnvalue_2 (Transformation|GetActorLocation _returnvalue))
  (bind _returnvalue_3 (- _returnvalue_2 "0.000000,0.000000,65.000000"))
  (:Pressed
    (bind _outhit (Collision|SphereTraceByChannel _returnvalue_3 _returnvalue_3 1.2e+02 "TraceTypeQuery1" false 0 "None"))
    (bind _asbp_item (Utilities|Casting|CastToBP_item (.HitActor (Collision|BreakHitResult _outhit))))
    (for (_array_element _array_index) (Variables|Default|Getitems)
      (Utilities|IsValid _asbp_item
        (:Is%20Valid
          (if (Math|Boolean|ANDBoolean (Utilities|Enum|Equal(Enum) (.Name (Utilities|Struct|BreakF_itemstructure _array_element)) (.Name (Utilities|Struct|BreakF_itemstructure (Variables|/Game/1TopDowm_UNIR/inventory/blueprits/BP_item.BP_item_C|Getitem _asbp_item)))) (.Stackeable (Utilities|Struct|BreakF_itemstructure (Variables|/Game/1TopDowm_UNIR/inventory/blueprits/BP_item.BP_item_C|Getitem _asbp_item))) (<= (+ (.quantity (Utilities|Struct|BreakF_itemstructure _array_element)) (.quantity (Utilities|Struct|BreakF_itemstructure (Variables|/Game/1TopDowm_UNIR/inventory/blueprits/BP_item.BP_item_C|Getitem _asbp_item)))) 64))
            (Utilities|Array|SetArrayElem (Variables|Default|Getitems) _array_index (Utilities|Struct|MakeF_itemstructure (.name (Variables|/Game/1TopDowm_UNIR/inventory/blueprits/BP_item.BP_item_C|Getitem _asbp_item)) (.stackeable (Variables|/Game/1TopDowm_UNIR/inventory/blueprits/BP_item.BP_item_C|Getitem _asbp_item)) (+ (.quantity (Utilities|Struct|BreakF_itemstructure _array_element)) (.quantity (Utilities|Struct|BreakF_itemstructure (Variables|/Game/1TopDowm_UNIR/inventory/blueprits/BP_item.BP_item_C|Getitem _asbp_item)))) (.thumnail (Variables|/Game/1TopDowm_UNIR/inventory/blueprits/BP_item.BP_item_C|Getitem _asbp_item)) (.mesh (Variables|/Game/1TopDowm_UNIR/inventory/blueprits/BP_item.BP_item_C|Getitem _asbp_item))))
            (Audio|SpawnSound2D "/Game/1TopDowm_UNIR/SFX/pickup.pickup" 1.0 1.0 0.0 0)
            (Default|LoadInventory (Variables|Default|Getwidgetinventory) self :!label _label)
            (Actor|DestroyActor _asbp_item)
            (elif (== (.quantity (Utilities|Struct|BreakF_itemstructure _array_element)) 0)
              (Utilities|Array|SetArrayElem (Variables|Default|Getitems) _array_index (Variables|/Game/1TopDowm_UNIR/inventory/blueprits/BP_item.BP_item_C|Getitem _asbp_item))
              (Audio|SpawnSound2D "/Game/1TopDowm_UNIR/SFX/pickup.pickup" 1.0 1.0 0.0 0)
              (goto _label))))))))