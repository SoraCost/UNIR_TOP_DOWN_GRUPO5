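; BP_door is a locked door in a top-down game that opens once the player holds every key in the level.
; On BeginPlay it counts all BP_key actors to set the required total.
; When the player character overlaps its Box, a matching key count destroys the Cube once via DoOnce.
; Otherwise it prints a Spanish debug message with the number of keys still missing.
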(event OnComponentBeginOverlap(Box)
  (params (OverlappedComponent :type Primitive%20Component%20Object%20Reference) (OtherActor :type Actor%20Object%20Reference) (OtherComp :type Primitive%20Component%20Object%20Reference) (OtherBodyIndex :type Integer) (bFromSweep :type Boolean) (SweepResult :type Hit%20Result%20Structure%20%28by%20ref%29))
  (bind _numtotalkeys (Variables|Default|GetNumTotalKeys))
  (bind _asbp_top_down_character_unir (Utilities|Casting|CastToBP_TopDown_Character_UNIR OtherActor))
  (bind _newparam (Default|GetNumKeys _asbp_top_down_character_unir))
  (if (== _newparam _numtotalkeys)
    (Utilities|FlowControl|DoOnce false
      (:Completed
        (Components|DestroyComponent (Variables|Default|GetCube))))
    (else
      (Development|PrintString (Utilities|String|Append "Te falta por recoger" (Utilities|String|ToString(Integer) (- _numtotalkeys _newparam)) "llave/s")))))

(event EventBeginPlay
  (bind _outactors (Actor|GetAllActorsOfClass "/Game/1TopDowm_UNIR/Blueprint/BP_key.BP_key_C"))
  (Variables|Default|SetNumTotalKeys (Utilities|Array|Length _outactors)))

(event Collision|EventActorBeginOverlap
  (params (OtherActor :type Actor%20Object%20Reference)))

(event EventTick
  (params (DeltaSeconds :type Float%20%28single-precision%29)))

(fn ConstructionScript)